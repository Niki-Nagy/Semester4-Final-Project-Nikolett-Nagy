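; BP_ScenarioTrigger is a world trigger that starts chat scenarios from an ordered sequence when the player presses E nearby.
; Its box overlap tracks whether the first-person character is in range, and BeginPlay caches the BP_Chatmanager found in the level.
; If unlocked and scenarios remain, E calls StartScenario with the current ID and itself as TriggerRef.
; AdvanceToNextScenario increments the sequence index, which this file never calls itself.
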(event `self.ReceiveBeginPlay`
  (bind _returnvalue (`GameplayStatics.GetActorOfClass` "/Game/Blueprints/ChatSystem/Managers/BP_Chatmanager.BP_Chatmanager_C"))
  (set `self.ChatManagerRef` _returnvalue))

(event `self.Box_Trigger.OnComponentBeginOverlap`
  (params (OverlappedComponent :type "PrimitiveComponent Object Reference") (OtherActor :type "Actor Object Reference") (OtherComp :type "PrimitiveComponent Object Reference") (OtherBodyIndex :type Integer) (bFromSweep :type Boolean) (SweepResult :type "HitResult Structure (by ref)"))
  (cast `/Game/FirstPerson/Blueprints/BP_FirstPersonCharacter` OtherActor)
  (set `self.bPlayerInRange` true))

(event `self.Box_Trigger.OnComponentEndOverlap`
  (params (OverlappedComponent :type "PrimitiveComponent Object Reference") (OtherActor :type "Actor Object Reference") (OtherComp :type "PrimitiveComponent Object Reference") (OtherBodyIndex :type Integer))
  (cast `/Game/FirstPerson/Blueprints/BP_FirstPersonCharacter` OtherActor)
  (set `self.bPlayerInRange` false))

(event `Key|E`
  (params (Key :type "Key Structure"))
  (bind _chatmanagerref (`self.ChatManagerRef`))
  (:`Pressed`
    (if (`self.bPlayerInRange`)
      (if (`self.bUnlocked`)
        (`/Engine/EditorBlueprintResources/StandardMacros.IsValid` _chatmanagerref
          (:`Is Valid`
            (if (< (`self.CurrentScenarioIndex`) (`KismetArrayLibrary.Array_Length` (`self.ScenarioSequence`)))
              (`/Game/Blueprints/ChatSystem/Managers/BP_Chatmanager.StartScenario` _chatmanagerref (`|GetArrayItem` (`self.ScenarioSequence`) (`self.CurrentScenarioIndex`)) self))))))))

(fn `AdvanceToNextScenario`
  (set `self.CurrentScenarioIndex` (+ (`self.CurrentScenarioIndex`) 1)))

(fn `UserConstructionScript`)