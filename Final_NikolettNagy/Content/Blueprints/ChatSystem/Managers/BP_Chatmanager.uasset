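; Chat manager that runs branching, data-table-driven message scenarios in a chat screen widget.
; StartScenario shows the UI, locks player movement and look, then loads dialogue nodes whose messages play through a queue with timed typing indicators.
; Node type decides whether to auto-advance, offer reaction choices or finish; a chosen reaction posts the player's reply and loads its next node.
; Finishing advances the calling trigger; closing chat restores game input.
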(event `self.ReceiveBeginPlay`)

(event `StartMessagePlayback`
  (if (== (`KismetArrayLibrary.Array_Length` (`self.PendingMessages`)) 0)
    (`self.HandleNodeFinished`)
    (else
      (`self.DisplayNextMessage`))))

(event `DisplayNextMessage`
  (bind (_currentmessage_messageid _currentmessage_sendername _currentmessage_messagetext _currentmessage_messagerole _currentmessage_delaybeforeshow _currentmessage_bplayerowned) (break `/Game/Blueprints/ChatSystem/Structs/S_ChatMessage` (`self.CurrentMessage`)))
  (bind (_currentmessage_messageid_2 _currentmessage_sendername_2 _currentmessage_messagetext_2) (break `/Game/Blueprints/ChatSystem/Structs/S_ChatMessage` (`self.CurrentMessage`)))
  (if (== (`KismetArrayLibrary.Array_Length` (`self.PendingMessages`)) 0)
    (`self.HandleNodeFinished`)
    (else
      (set `self.CurrentMessage` (`|GetArrayItem` (`self.PendingMessages`)))
      (`KismetArrayLibrary.Array_Remove` (`self.PendingMessages`))
      (`/Game/Blueprints/ChatSystem/Widgets/WBP_ChatScreen.ShowTypingIndicator` (`self.ChatScreenRef`) _currentmessage_bplayerowned)
      (`KismetSystemLibrary.K2_SetTimerDelegate` (`|CreateDelegate` :!event `ShowCurrentMessageAfterTyping`) (`KismetMathLibrary.Conv_IntToDouble` (`KismetMathLibrary.Clamp` (`KismetMathLibrary.FTrunc` (* (`KismetMathLibrary.Conv_IntToDouble` (`KismetStringLibrary.Len` (`KismetTextLibrary.Conv_TextToString` _currentmessage_messagetext_2))) 0.03)) 0 1))))))

(event `HandleMessageDisplayed`
  (if (> (`KismetArrayLibrary.Array_Length` (`self.PendingMessages`)) 0)
    (`self.DisplayNextMessage`)
    (else
      (`self.HandleNodeFinished`))))

(event `HandleNodeFinished`
  (bind _noderow (`self.GetNodeRow` (`self.CurrentNodeID`)))
  (switch `/Game/Blueprints/ChatSystem/Enums/E_NodeType` (`.Nodetype_5_D762B670409E435CE09E8B99D2A7198D` (break `/Game/Blueprints/ChatSystem/Structs/S_DialogueNode` _noderow))
    (:`NewEnumerator0`
      (if (`.bAutoAdvance_16_B985D2584FB9746E6EAA4EAC75F0DBB7` (break `/Game/Blueprints/ChatSystem/Structs/S_DialogueNode` _noderow))
        (`KismetSystemLibrary.K2_SetTimerDelegate` :`Time` (`.AutoAdvanceDelay_22_35BF26A741ED5C4430D7A1A7A2E43C90` (break `/Game/Blueprints/ChatSystem/Structs/S_DialogueNode` _noderow)))
        (`self.LoadNode` (`.NextNodeIfAuto_19_4A284752475EAD3E5D73E195970B007C` (break `/Game/Blueprints/ChatSystem/Structs/S_DialogueNode` _noderow)))
        (else
          (`self.FinishScenario`))))
    (:`NewEnumerator1`
      (set `self.CurrentState` "NewEnumerator3")
      (`/Game/Blueprints/ChatSystem/Widgets/WBP_ChatScreen.ShowReactionChoices` (`self.ChatScreenRef`) (`self.CurrentChoices`)))
    (:`NewEnumerator2`
      (if (`.bAutoAdvance_16_B985D2584FB9746E6EAA4EAC75F0DBB7` (break `/Game/Blueprints/ChatSystem/Structs/S_DialogueNode` _noderow))
        (`KismetSystemLibrary.K2_SetTimerDelegate` :`Time` (`.AutoAdvanceDelay_22_35BF26A741ED5C4430D7A1A7A2E43C90` (break `/Game/Blueprints/ChatSystem/Structs/S_DialogueNode` _noderow)))
        (`self.LoadNode` (`.NextNodeIfAuto_19_4A284752475EAD3E5D73E195970B007C` (break `/Game/Blueprints/ChatSystem/Structs/S_DialogueNode` _noderow)))
        (else
          (`self.FinishScenario`))))
    (:`NewEnumerator3`
      (`self.FinishScenario`))))

(event `ShowCurrentReactionChoices`
  (`/Game/Blueprints/ChatSystem/Widgets/WBP_ChatScreen.ShowReactionChoices` :`self` (`self.ChatScreenRef`)))

(event `HandleReactionSelected`
  (params (SelectedChoice :type "/Game/Blueprints/ChatSystem/Structs/S_ReactionChoice Structure"))
  (if (`|EnumEquality` (`self.CurrentState`) "NewEnumerator3")
    (set `self.CurrentState` "NewEnumerator4")
    (set `self.LastSelectedChoice` SelectedChoice)
    (`/Game/Blueprints/ChatSystem/Widgets/WBP_ChatScreen.DisableReactionChoices` (`self.ChatScreenRef`))
    (`self.InsertPlayerReplyThenAdvance`)))

(event `InsertPlayerReplyThenAdvance`
  (bind (_lastselectedchoice_choiceid _lastselectedchoice_buttonlabel _lastselectedchoice_reactiontype _lastselectedchoice_playerreplytext) (break `/Game/Blueprints/ChatSystem/Structs/S_ReactionChoice` (`self.LastSelectedChoice`)))
  (set `self.PendingPlayerReplyMessage` (make `/Game/Blueprints/ChatSystem/Structs/S_ChatMessage` "PlayerReply" "You" _lastselectedchoice_playerreplytext "NewEnumerator0" 0.2 true false false null))
  (`KismetSystemLibrary.K2_SetTimerDelegate` (`|CreateDelegate` :!event `ShowPlayerReplyInAdvance`) 0.2))

(event `OnTakeAnyDamage_Event` :!signature `self.OnTakeAnyDamage`
  (params (DamagedActor :type "Actor Object Reference") (Damage :type "Float (single-precision)") (DamageType :type "DamageType Object Reference") (InstigatedBy :type "Controller Object Reference") (DamageCauser :type "Actor Object Reference")))

(event `ShowCurrentMessage`
  (`/Game/Blueprints/ChatSystem/Widgets/WBP_ChatScreen.AddChatMessage` (`self.ChatScreenRef`) (`self.CurrentMessage`))
  (`self.HandleMessageDisplayed`))

(event `ShowPlayerReplyInAdvance`
  (bind (_lastselectedchoice_choiceid _lastselectedchoice_buttonlabel _lastselectedchoice_reactiontype _lastselectedchoice_playerreplytext _lastselectedchoice_nextnodeid) (break `/Game/Blueprints/ChatSystem/Structs/S_ReactionChoice` (`self.LastSelectedChoice`)))
  (`/Game/Blueprints/ChatSystem/Widgets/WBP_ChatScreen.AddChatMessage` (`self.ChatScreenRef`) (`self.PendingPlayerReplyMessage`))
  (`self.LoadNode` _lastselectedchoice_nextnodeid))

(event `HandleCloseChatRequested`
  (bind _returnvalue (`GameplayStatics.GetPlayerController` 0))
  (`/Game/Blueprints/ChatSystem/Widgets/WBP_ChatScreen.HideChatUI` (`self.ChatScreenRef`))
  (`WidgetBlueprintLibrary.SetInputMode_GameOnly` _returnvalue)
  (set `PlayerController.bShowMouseCursor` false _returnvalue)
  (`Controller.SetIgnoreMoveInput` _returnvalue false)
  (`Controller.SetIgnoreLookInput` _returnvalue false)
  (`/Game/Blueprints/ChatSystem/Widgets/WBP_ChatScreen.HideTypingIndicator` (`self.ChatScreenRef`)))

(event `ShowCurrentMessageAfterTyping`
  (`/Game/Blueprints/ChatSystem/Widgets/WBP_ChatScreen.HideTypingIndicator` (`self.ChatScreenRef`))
  (`self.ShowCurrentMessage`)
  (`self.HandleMessageDisplayed`))

(fn `ContinueStartScenario`
  (bind _currentscenarioid (`self.CurrentScenarioID`))
  (`/Game/Blueprints/ChatSystem/Widgets/WBP_ChatScreen.ClearChat` (`self.ChatScreenRef`))
  (`KismetSystemLibrary.PrintString` (`KismetStringLibrary.Conv_NameToString` _currentscenarioid))
  (bind _scenariorow (`self.GetScenarioRow` _currentscenarioid))
  (`self.LoadNode` (`.StartNodeID_8_4D1001FC4BC2CCA41A665A92197199EB` (break `/Game/Blueprints/ChatSystem/Structs/S_ScenarioDefinition` _scenariorow))))

(fn `FinishScenario`
  (bind _currenttriggerref (`self.CurrentTriggerRef`))
  (set `self.CurrentState` "NewEnumerator5")
  (`/Engine/EditorBlueprintResources/StandardMacros.IsValid` _currenttriggerref
    (:`Is Valid`
      (`/Game/Blueprints/ChatSystem/BP_ScenarioTrigger.AdvanceToNextScenario` _currenttriggerref)
      (set `self.bScenarioRunning` false)
      (`/Game/Blueprints/ChatSystem/Widgets/WBP_ChatScreen.HideTypingIndicator` (`self.ChatScreenRef`)))
    (:`Is Not Valid`
      (`KismetSystemLibrary.PrintString` "No more scenarios"))))

(fn `GetNodeRow`
  (params (NodeID :type Name))
  (returns (NodeRow :type "/Game/Blueprints/ChatSystem/Structs/S_DialogueNode Structure"))
  (bind _returnvalue (`|GetDataTableRow` "/Game/Blueprints/ChatSystem/Data/DT_DialogueNodes.DT_DialogueNodes" NodeID)
    (:`then`
      (return _returnvalue))))

(fn `GetScenarioRow`
  (params (ScenarioID :type Name))
  (returns (ScenarioRow :type "/Game/Blueprints/ChatSystem/Structs/S_ScenarioDefinition Structure"))
  (bind _returnvalue (`|GetDataTableRow` (`self.ScenariosTable`) ScenarioID)
    (:`then`
      (return _returnvalue))))

(fn `LoadNode`
  (params (NodeID :type Name))
  (set `self.CurrentState` "NewEnumerator1")
  (bind _output_get (set `self.CurrentNodeID` NodeID))
  (bind _noderow (`self.GetNodeRow` _output_get))
  (set `self.PendingMessages` (`.Messages_9_2497449E41595051A87C8C9E8EE99D95` (break `/Game/Blueprints/ChatSystem/Structs/S_DialogueNode` _noderow)))
  (set `self.CurrentChoices` (`.ReactionChoices_12_5A42FEE042A47AF23C1B319FF440CDA9` (break `/Game/Blueprints/ChatSystem/Structs/S_DialogueNode` _noderow)))
  (`/Game/Blueprints/ChatSystem/Widgets/WBP_ChatScreen.HideReactionChocies` (`self.ChatScreenRef`))
  (set `self.CurrentState` "NewEnumerator2")
  (`self.StartMessagePlayback`))

(fn `ResetScenarioState`
  (bind _chatscreenref (`self.ChatScreenRef`))
  (`KismetArrayLibrary.Array_Clear` (`self.PendingMessages`))
  (`KismetArrayLibrary.Array_Clear` (`self.CurrentChoices`))
  (set `self.CurrentNodeID` "None")
  (set `self.CurrentState` "NewEnumerator0")
  (`/Engine/EditorBlueprintResources/StandardMacros.IsValid` _chatscreenref
    (:`Is Valid`
      (`/Game/Blueprints/ChatSystem/Widgets/WBP_ChatScreen.ClearChat` _chatscreenref))))

(fn `StartScenario`
  (params (ScenarioID :type Name) (TriggerRef :type "/Game/Blueprints/ChatSystem/BP_ScenarioTrigger Object Reference"))
  (bind _returnvalue (`GameplayStatics.GetPlayerController` 0))
  (bind _returnvalue_2 (`GameplayStatics.GetPlayerController` 0))
  (bind _chatscreenref (`self.ChatScreenRef`))
  (if (not (`self.bScenarioRunning`))
    (set `self.bScenarioRunning` true)
    (set `self.CurrentScenarioID` ScenarioID)
    (set `self.CurrentTriggerRef` TriggerRef)
    (`self.ResetScenarioState`)
    (`/Engine/EditorBlueprintResources/StandardMacros.IsValid` (`self.ChatScreenRef`)
      (:`Is Valid`
        (`/Game/Blueprints/ChatSystem/Widgets/WBP_ChatScreen.ShowChatUI` (`self.ChatScreenRef`))
        (set `PlayerController.bShowMouseCursor` true _returnvalue_2)
        (`WidgetBlueprintLibrary.SetInputMode_UIOnlyEx` _returnvalue_2 _chatscreenref)
        (`Controller.SetIgnoreMoveInput` _returnvalue_2 true)
        (`Controller.SetIgnoreLookInput` _returnvalue_2 true)
        (`self.ContinueStartScenario`))
      (:`Is Not Valid`
        (bind _returnvalue_3 (`|CreateWidget` "/Game/Blueprints/ChatSystem/Widgets/WBP_ChatScreen.WBP_ChatScreen_C" (`GameplayStatics.GetPlayerController` 0)))
        (bind _output_get (set `self.ChatScreenRef` _returnvalue_3))
        (`UserWidget.AddToViewport` _output_get 0)
        (`/Game/Blueprints/ChatSystem/Widgets/WBP_ChatScreen.ShowChatUI` _chatscreenref)
        (set `PlayerController.bShowMouseCursor` true _returnvalue)
        (`WidgetBlueprintLibrary.SetInputMode_UIOnlyEx` _returnvalue _chatscreenref)
        (`Controller.SetIgnoreMoveInput` _returnvalue true)
        (`Controller.SetIgnoreLookInput` _returnvalue true)
        (add `/Game/Blueprints/ChatSystem/Widgets/WBP_ChatScreen.OnReactionSelected` (`self.ChatScreenRef`) (`|CreateDelegate` :!event `HandleReactionSelected`))
        (add `/Game/Blueprints/ChatSystem/Widgets/WBP_ChatScreen.OnCloseChatRequested` (`self.ChatScreenRef`) (`|CreateDelegate` :!event `HandleCloseChatRequested`))
        (`self.ContinueStartScenario`)))))

(fn `UserConstructionScript`)