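; BP_RoomLightController is a chat system actor that switches a room's lighting between positive, neutral and negative moods.
; Three functions each set the intensity and color of PointLightMain, from bright warm orange through near-white to dimmer cool blue.
; It has no active event or construction logic, so the mood changes only when one of these functions is called.
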(fn `SetNegativeMood`
  (`LightComponent.SetIntensity` (`self.PointLight_Main`) 2500.0)
  (`LightComponent.SetLightColor` (`self.PointLight_Main`) (struct :`R` 0.176 :`G` 0.726781 :`B` 1.0 :`A` 1.0) true))

(fn `SetNeutralMood`
  (`LightComponent.SetIntensity` (`self.PointLight_Main`) 4000.0)
  (`LightComponent.SetLightColor` (`self.PointLight_Main`) (struct :`R` 0.914 :`G` 1.0 :`B` 0.964016 :`A` 1.0) true))

(fn `SetPositiveMood`
  (`LightComponent.SetIntensity` (`self.PointLight_Main`) 6000.0)
  (`LightComponent.SetLightColor` (`self.PointLight_Main`) (struct :`R` 0.794003 :`G` 0.156704 :`A` 1.0) true))

(fn `UserConstructionScript`)