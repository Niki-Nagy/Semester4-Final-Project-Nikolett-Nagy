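; BP_Comm is an interactable comms terminal that highlights on first-person character overlap and opens a communications UI.
; A Box overlap toggles the Caninteract flag, though Interact does not check it.
; Interact creates WBP_Comms with a self-reference, switches to UI-only input focused on CommsWidgetRef (never assigned here), and locks movement and look.
; Positive, neutral and negative feedback events set a referenced light's intensity to signal the outcome.
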(event `self.ReceiveBeginPlay`
  (`self.EnableInput` (`GameplayStatics.GetPlayerController` 0)))

(event `self.Terminal.OnComponentBeginOverlap`
  (params (OverlappedComponent :type "PrimitiveComponent Object Reference") (OtherActor :type "Actor Object Reference") (OtherComp :type "PrimitiveComponent Object Reference") (OtherBodyIndex :type Integer) (bFromSweep :type Boolean) (SweepResult :type "HitResult Structure (by ref)"))
  (cast `/Game/FirstPerson/Blueprints/BP_FirstPersonCharacter` OtherActor)
  (`PrimitiveComponent.SetMaterial` (`self.Terminal`) 0 "/Game/Materials/M_Terminal_highlight.M_Terminal_highlight"))

(event `self.Box.OnComponentBeginOverlap`
  (params (OverlappedComponent :type "PrimitiveComponent Object Reference") (OtherActor :type "Actor Object Reference") (OtherComp :type "PrimitiveComponent Object Reference") (OtherBodyIndex :type Integer) (bFromSweep :type Boolean) (SweepResult :type "HitResult Structure (by ref)"))
  (cast `/Game/FirstPerson/Blueprints/BP_FirstPersonCharacter` OtherActor)
  (set `self.Caninteract` true))

(event `self.Box.OnComponentEndOverlap`
  (params (OverlappedComponent :type "PrimitiveComponent Object Reference") (OtherActor :type "Actor Object Reference") (OtherComp :type "PrimitiveComponent Object Reference") (OtherBodyIndex :type Integer))
  (cast `/Game/FirstPerson/Blueprints/BP_FirstPersonCharacter` OtherActor)
  (set `self.Caninteract` false))

(event `Interact`
  (bind _returnvalue (`GameplayStatics.GetPlayerController` 0))
  (`KismetSystemLibrary.PrintString` "Terminal interacted")
  (bind _returnvalue_2 (`|CreateWidget` "/Game/Blueprints/WBP_Comms.WBP_Comms_C" null self))
  (`UserWidget.AddToViewport` _returnvalue_2 0)
  (`WidgetBlueprintLibrary.SetInputMode_UIOnlyEx` _returnvalue (`self.CommsWidgetRef`))
  (`Controller.SetIgnoreMoveInput` _returnvalue true)
  (`Controller.SetIgnoreLookInput` _returnvalue true)
  (set `PlayerController.bShowMouseCursor` true (`GameplayStatics.GetPlayerController` 0)))

(event `ApplyPositiveFeedback`
  (`/Engine/EditorBlueprintResources/StandardMacros.IsValid` (`self.LightRef`)
    (:`Is Valid`
      (`LightComponent.SetIntensity` (`Light.LightComponent` (`self.LightRef`)) 6500.0)
      (`KismetSystemLibrary.PrintString` "POS"))))

(event `NeutralFeedback`
  (`/Engine/EditorBlueprintResources/StandardMacros.IsValid` (`self.LightRef`)
    (:`Is Valid`
      (`LightComponent.SetIntensity` (`Light.LightComponent` (`self.LightRef`)) 5000.0)
      (`KismetSystemLibrary.PrintString` "NEU"))))

(event `NegativeFeedback`
  (`/Engine/EditorBlueprintResources/StandardMacros.IsValid` (`self.LightRef`)
    (:`Is Valid`
      (`LightComponent.SetIntensity` (`Light.LightComponent` (`self.LightRef`)) 1000.0)
      (`KismetSystemLibrary.PrintString` "NEG"))))

(fn `UserConstructionScript`)